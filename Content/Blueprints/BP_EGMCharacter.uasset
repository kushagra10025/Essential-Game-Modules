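; BP_EGMCharacter is a player character with movement, look and interaction controls driven by Enhanced Input.
; BeginPlay sets up the NPIMACInteractionTrace component and adds the IMC_Movement mapping context to player 0.
; Move actions apply input along the capsule's forward and right vectors, while look actions feed controller pitch and yaw.
; IA_Interact forwards its press and release to the trace component's TryToInteract as true and false.
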(event Input|EnhancedActionEvents|EnhancedInputActionIA_MoveForwards
  (params (ActionValue :type Float%20%28double-precision%29) (ElapsedSeconds :type Float%20%28double-precision%29) (TriggeredSeconds :type Float%20%28double-precision%29) (InputAction :type Input%20Action%20Object%20Reference :default "/Game/Inputs/IA_MoveForwards.IA_MoveForwards"))
  (:Triggered
    (Pawn|Input|AddMovementInput (Math|Vector|GetForwardVector (Variables|Collision|GetCapsuleComponent)) ActionValue false :!label _label))
  (:Completed
    (goto _label)))

(event Input|EnhancedActionEvents|EnhancedInputActionIA_MoveRight
  (params (ActionValue :type Float%20%28double-precision%29) (ElapsedSeconds :type Float%20%28double-precision%29) (TriggeredSeconds :type Float%20%28double-precision%29) (InputAction :type Input%20Action%20Object%20Reference :default "/Game/Inputs/IA_MoveRight.IA_MoveRight"))
  (:Triggered
    (Pawn|Input|AddMovementInput (Math|Vector|GetRightVector (Variables|Collision|GetCapsuleComponent)) ActionValue false :!label _label))
  (:Completed
    (goto _label)))

(event Input|EnhancedActionEvents|EnhancedInputActionIA_LookUp
  (params (ActionValue :type Float%20%28double-precision%29) (ElapsedSeconds :type Float%20%28double-precision%29) (TriggeredSeconds :type Float%20%28double-precision%29) (InputAction :type Input%20Action%20Object%20Reference :default "/Game/Inputs/IA_LookUp.IA_LookUp"))
  (:Triggered
    (Pawn|Input|AddControllerPitchInput ActionValue :!label _label))
  (:Completed
    (goto _label)))

(event Input|EnhancedActionEvents|EnhancedInputActionIA_LookRight
  (params (ActionValue :type Float%20%28double-precision%29) (ElapsedSeconds :type Float%20%28double-precision%29) (TriggeredSeconds :type Float%20%28double-precision%29) (InputAction :type Input%20Action%20Object%20Reference :default "/Game/Inputs/IA_LookRight.IA_LookRight"))
  (:Triggered
    (Pawn|Input|AddControllerYawInput ActionValue :!label _label))
  (:Completed
    (goto _label)))

(event Input|EnhancedActionEvents|EnhancedInputActionIA_Interact
  (params (ActionValue :type Boolean) (ElapsedSeconds :type Float%20%28double-precision%29) (TriggeredSeconds :type Float%20%28double-precision%29) (InputAction :type Input%20Action%20Object%20Reference :default "/Game/Inputs/IA_Interact.IA_Interact"))
  (bind _npim_ac_interactiontrace (Variables|Default|GetNPIM_AC_InteractionTrace))
  (:Started
    (Class|NPIMACInteractionTrace|TrytoInteract _npim_ac_interactiontrace true))
  (:Completed
    (Class|NPIMACInteractionTrace|TrytoInteract _npim_ac_interactiontrace false)))

(event EventBeginPlay
  (Class|NPIMACInteractionTrace|SetupInteractionTrace (Variables|Default|GetNPIM_AC_InteractionTrace))
  (Input|AddMappingContext (PlayerController|LocalPlayerSubsystems|GetEnhancedInputLocalPlayerSubsystem (Game|GetPlayerController 0)) "/Game/Inputs/IMC_Movement.IMC_Movement" 0 "(bIgnoreAllPressedKeysUntilRelease=True,bForceImmediately=False)"))

(fn ConstructionScript)